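; Debug probe actor for testing KhazanCharacter's locomotion movement policy through number keys.
; BeginPlay enables input for a valid TargetCharacter or a KhazanCharacter player pawn, though that fallback sets TargetCharacter to None.
; Key 0 prints intent and resolved-policy snapshots alongside CharacterMovement's max walk speed.
; Key 1 replaces a handle-based constraint capping gait at Run, and key 2 releases it.
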(event EventBeginPlay
  (bind _returnvalue (Game|GetPlayerController 0))
  (if (Utilities|IsValid (Variables|Default|GetTargetCharacter))
    (Input|EnableInput _returnvalue)
    (else
      (Utilities|Casting|CastToKhazanCharacter (Game|GetPlayerCharacter 0)
        (:then
          (Variables|Default|SetTargetCharacter 0)
          (Input|EnableInput _returnvalue))
        (:CastFailed
          (Development|PrintString "M2 Probe: TargetCharacter not found"))))))

(event Collision|EventActorBeginOverlap
  (params (OtherActor :type Actor%20Object%20Reference)))

(event EventTick
  (params (DeltaSeconds :type Float%20%28single-precision%29)))

(event Input|KeyboardEvents|0
  (params (Key :type Key%20Structure :default "None"))
  (bind _targetcharacter (Variables|Default|GetTargetCharacter))
  (bind _returnvalue (Class|KhazanCharacter|GetLocomotionComponent _targetcharacter))
  (bind _returnvalue_2 (Class|KhazanLocomotionComponent|GetLocomotionIntentSnapshot _returnvalue))
  (bind _returnvalue_3 (Class|KhazanLocomotionComponent|GetResolvedMovementPolicySnapshot _returnvalue))
  (bind (_moveinputworld _inputamount _requestedgait) (Utilities|Struct|BreakKhazanLocomotionIntent _returnvalue_2))
  (bind (_bmovementallowedbytags _maxallowedgait _resolvedgait _resolvedrotationmode _maxwalkspeed) (Utilities|Struct|BreakKhazanResolvedMovementPolicy _returnvalue_3))
  (:Pressed
    (Development|PrintString (Utilities|String|ToString(Text) (Utilities|Text|FormatText "Input={InputAmount} 
Requested={RequestedGait} 
MaxAllowed={MaxAllowedGait} 
Resolved={ResolvedGait} 
Rotation={ResolvedRotationMode} 
TagAllowed={bMovementAllowedByTags} 
PolicyMax={Policy.MaxWalkSpeed} 
CMCMax={CharacterMovement.MaxWalkSpeed} 
Speed2D={VectorLengthXY(TargetCharacter.Velocity)}" _inputamount (Utilities|String|EnumtoString _requestedgait) (Utilities|String|EnumtoString _maxallowedgait) (Utilities|String|EnumtoString _resolvedgait) (Utilities|String|EnumtoString _resolvedrotationmode) _bmovementallowedbytags _maxwalkspeed (Variables|/Script/Engine.CharacterMovementComponent|GetMaxWalkSpeed (Variables|/Script/Engine.Character|GetCharacterMovement (Variables|Default|GetTargetCharacter))))))))

(event Input|KeyboardEvents|1
  (params (Key :type Key%20Structure :default "None"))
  (bind _targetcharacter (Variables|Default|GetTargetCharacter))
  (bind _returnvalue (Class|KhazanCharacter|GetLocomotionComponent _targetcharacter))
  (:Pressed
    (Class|KhazanLocomotionComponent|ReleaseMovementConstraint _returnvalue (Variables|Default|GetGaitHandleA))
    (bind _returnvalue_2 (Class|KhazanLocomotionComponent|AcquireMovementConstraint _returnvalue self (Utilities|Struct|MakeKhazanMovementConstraint "Run" false "VelocityDirection" 0 "Test.Gait.A")))
    (Variables|Default|SetGaitHandleA _returnvalue_2)))

(event Input|KeyboardEvents|2
  (params (Key :type Key%20Structure :default "None"))
  (:Pressed
    (Class|KhazanLocomotionComponent|ReleaseMovementConstraint (Class|KhazanCharacter|GetLocomotionComponent (Variables|Default|GetTargetCharacter)) (Variables|Default|GetGaitHandleA))))

(fn ConstructionScript)