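; BP_Slash_twice is a slash VFX actor that repeatedly plays a two-attack animation sequence with slash effects.
; From BeginPlay, a timed chain plays Attack_B_Fast, waits for a Duration variable, then plays Attack_A_Fast on the skeletal mesh.
; As the second animation starts, it resets and activates NSSlash, then NSSlash2 shortly after.
; The custom event calls itself after a delay, so the sequence loops indefinitely.
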(event Custom|CustomEvent
  (bind _skeletalmesh (Variables|Default|GetSkeletalMesh))
  (Utilities|FlowControl|Delay 1.0)
  (Components|Animation|PlayAnimation _skeletalmesh "/Game/VFX/03_SlashHit/Demo/Attack_B_Fast.Attack_B_Fast" false)
  (Utilities|FlowControl|Delay (Variables|Default|GetDuration))
  (Components|Animation|PlayAnimation _skeletalmesh "/Game/VFX/03_SlashHit/Demo/Attack_A_Fast.Attack_A_Fast" false)
  (Components|Activation|SetActive (Variables|Default|GetNS_Slash) true true)
  (Utilities|FlowControl|Delay 0.1)
  (Components|Activation|SetActive (Variables|Default|GetNS_Slash2) true true)
  (Utilities|FlowControl|Delay 1.0)
  (CallFunction|CustomEvent))

(event EventBeginPlay
  (bind _skeletalmesh (Variables|Default|GetSkeletalMesh))
  (Utilities|FlowControl|Delay 1.0)
  (Components|Animation|PlayAnimation _skeletalmesh "/Game/VFX/03_SlashHit/Demo/Attack_B_Fast.Attack_B_Fast" false)
  (Utilities|FlowControl|Delay (Variables|Default|GetDuration))
  (Components|Animation|PlayAnimation _skeletalmesh "/Game/VFX/03_SlashHit/Demo/Attack_A_Fast.Attack_A_Fast" false)
  (Components|Activation|SetActive (Variables|Default|GetNS_Slash) true true)
  (Utilities|FlowControl|Delay 0.1)
  (Components|Activation|SetActive (Variables|Default|GetNS_Slash2) true true)
  (Utilities|FlowControl|Delay 1.0)
  (CallFunction|CustomEvent))

(fn ConstructionScript)