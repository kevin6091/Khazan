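; BP_Slash_Basic is an actor that repeatedly plays a slash attack animation with its VFX, apparently as an effect showcase.
; From BeginPlay, a delay-timed chain plays Ability_R on the skeletal mesh, then resets and activates NSSlash01 after the Duration variable elapses.
; NSBottomSpark follows shortly after, then the custom event calls itself after a pause, looping the sequence indefinitely.
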(event Custom|CustomEvent
  (Utilities|FlowControl|Delay 1.0)
  (Components|Animation|PlayAnimation (Variables|Default|GetSkeletalMesh) "/Game/VFX/03_SlashHit/Demo/Ability_R.Ability_R" false)
  (Utilities|FlowControl|Delay (Variables|Default|GetDuration))
  (Components|Activation|SetActive (Variables|Default|GetNS_Slash_01) true true)
  (Utilities|FlowControl|Delay 0.1)
  (Components|Activation|SetActive (Variables|Default|GetNS_BottomSpark) true true)
  (Utilities|FlowControl|Delay 1.0)
  (CallFunction|CustomEvent))

(event EventBeginPlay
  (Utilities|FlowControl|Delay 1.0)
  (Components|Animation|PlayAnimation (Variables|Default|GetSkeletalMesh) "/Game/VFX/03_SlashHit/Demo/Ability_R.Ability_R" false)
  (Utilities|FlowControl|Delay (Variables|Default|GetDuration))
  (Components|Activation|SetActive (Variables|Default|GetNS_Slash_01) true true)
  (Utilities|FlowControl|Delay 0.1)
  (Components|Activation|SetActive (Variables|Default|GetNS_BottomSpark) true true)
  (Utilities|FlowControl|Delay 1.0)
  (CallFunction|CustomEvent))

(event Collision|EventActorBeginOverlap
  (params (OtherActor :type Actor%20Object%20Reference)))

(event EventTick
  (params (DeltaSeconds :type Float%20%28single-precision%29)))

(fn ConstructionScript)