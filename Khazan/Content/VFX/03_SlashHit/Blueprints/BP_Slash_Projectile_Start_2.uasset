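; BP_Slash_Projectile_Start_2 is a VFX actor that repeatedly fires a slash projectile in sync with a character animation.
; From BeginPlay it loops: it waits, plays the Ability_E animation on its skeletal mesh, waits for Duration, then spawns SlashProjectile.
; The projectile takes the actor's rotation and its position plus an unrotated Location offset, and the cycle restarts through a self-calling custom event.
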(event Custom|CustomEvent
  (bind _returnvalue (Transformation|GetActorTransform))
  (Utilities|FlowControl|Delay 1.0)
  (Components|Animation|PlayAnimation (Variables|Default|GetSkeletalMesh) "/Game/VFX/03_SlashHit/Demo/Ability_E.Ability_E" false)
  (Utilities|FlowControl|Delay (Variables|Default|GetDuration))
  (Game|SpawnActorfromClass (Variables|Default|GetSlash_Projectile) (Math|Transform|MakeTransform (+ (.location _returnvalue) (Variables|Default|Getlocation)) (.rotation _returnvalue) "1.000000,1.000000,1.000000") "Undefined" "MultiplyWithRoot" 0 0)
  (Utilities|FlowControl|Delay 1.0)
  (CallFunction|CustomEvent))

(event EventBeginPlay
  (bind _returnvalue (Transformation|GetActorTransform))
  (Utilities|FlowControl|Delay 1.0)
  (Components|Animation|PlayAnimation (Variables|Default|GetSkeletalMesh) "/Game/VFX/03_SlashHit/Demo/Ability_E.Ability_E" false)
  (Utilities|FlowControl|Delay (Variables|Default|GetDuration))
  (Game|SpawnActorfromClass (Variables|Default|GetSlash_Projectile) (Math|Transform|MakeTransform (+ (.location _returnvalue) (Variables|Default|Getlocation)) (.rotation _returnvalue) "1.000000,1.000000,1.000000") "Undefined" "MultiplyWithRoot" 0 0)
  (Utilities|FlowControl|Delay 1.0)
  (CallFunction|CustomEvent))

(event Collision|EventActorBeginOverlap
  (params (OtherActor :type Actor%20Object%20Reference)))

(event EventTick
  (params (DeltaSeconds :type Float%20%28single-precision%29)))

(fn ConstructionScript)