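; Khazan player character Blueprint, currently holding a BeginPlay test of Gameplay Ability System movement blocking.
; It caches its Ability System Component and prints whether it is valid.
; It applies GE_Test_BlockMovement to itself twice, storing separate handles, then immediately removes both by handle with no delay between steps.
; The construction script is empty, and the graph contains no other gameplay logic.
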(event EventBeginPlay
  (bind _output_get (Variables|Default|SetTestASC (Ability|GetAbilitySystemComponent 0)))
  (Development|PrintString (Utilities|String|ToString(Boolean) (Utilities|IsValid _output_get)) (Utilities|IsValid _output_get))
  (Utilities|FlowControl|Sequence
    (:then_0
      (bind _returnvalue (GameplayEffects|ApplyGameplayEffectSpecToSelf (Variables|Default|GetTestASC) (GameplayEffects|MakeOutgoingSpec (Variables|Default|GetTestASC) "/Game/Test/GE_Test_BlockMovement.GE_Test_BlockMovement_C" 1.0 (GameplayEffects|MakeEffectContext (Variables|Default|GetTestASC)))))
      (Variables|Default|SetBlockHandleA _returnvalue))
    (:then_1
      (bind _returnvalue_2 (GameplayEffects|ApplyGameplayEffectSpecToSelf (Variables|Default|GetTestASC) (GameplayEffects|MakeOutgoingSpec (Variables|Default|GetTestASC) "/Game/Test/GE_Test_BlockMovement.GE_Test_BlockMovement_C" 1.0 (GameplayEffects|MakeEffectContext (Variables|Default|GetTestASC)))))
      (Variables|Default|SetBlockHandleB _returnvalue_2)
      (GameplayEffects|RemoveActiveGameplayEffect (Variables|Default|GetTestASC) (Variables|Default|GetBlockHandleA) -1)
      (GameplayEffects|RemoveActiveGameplayEffect (Variables|Default|GetTestASC) (Variables|Default|GetBlockHandleB) -1))))

(fn ConstructionScript)